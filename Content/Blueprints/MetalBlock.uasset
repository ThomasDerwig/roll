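; MetalBlock is a placeable metal building block that the player positions with the mouse and that breaks under too much weight.
; Clicking toggles dragging along the deprojected cursor ray, with the wheel setting depth and keys handling three-axis rotation or deletion.
; Material swaps signal hover and overlaps, ignoring certain helper classes.
; RegisterHit and RegisterUnhit track load; exceeding BreakLimit on a hit destroys the block and calls the HUD's fail message.
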(event `/Game/Interaction/Hit.Register unhit`
  (params (weight :type Integer))
  ;[1 1 1] Break
  (set `self.Current break` (- (`self.Current break`) weight))
  (`KismetSystemLibrary.PrintString` (`KismetStringLibrary.Conv_IntToString` (`self.Current break`))))

(event `Key|Delete`
  (params (Key :type "Key Structure"))
  ;[1 1 1] Delete NOTE: EVERY BLOCK SHOULD HAVE ITS OWN REMOVE MESSAGE BECAUSE OF COST
  (:`Pressed`
    (bind _asmy_hud (cast `/Game/HUD/MyHUD` (`PlayerController.GetHUD` (`GameplayStatics.GetPlayerController` 0))))
    (bind _asmain_hud (cast `/Game/HUD/MainHUD` (`/Game/HUD/MyHUD.widget` _asmy_hud)))
    (message `/Game/Interaction/remove.removeMBlock` _asmain_hud)
    (`self.K2_DestroyActor`)))

(event `/Game/Interaction/Hit.Register hit`
  (params (Weight :type Integer))
  ;[1 1 1] Break
  (set `self.Current break` (+ Weight (`self.Current break`)))
  (`KismetSystemLibrary.PrintString` (`KismetStringLibrary.Conv_IntToString` (`self.Current break`)))
  (`KismetSystemLibrary.Delay` 0.5)
  (if (> (`self.Current break`) (`self.Break Limit`))
    (`KismetSystemLibrary.Delay` 0.5)
    (`PrimitiveComponent.SetMaterial` (`self.Cube`) 0 "/Game/StarterContent/Materials/RedMetal.RedMetal")
    (`KismetSystemLibrary.Delay` 0.5)
    (`GameplayStatics.PlaySound2D` "/Game/Audio/MUST_USE_THIS_SOUND_EFFECT___WOOD_BREAKING_SOUND_EFFECT_-_MUST_USE_.MUST_USE_THIS_SOUND_EFFECT___WOOD_BREAKING_SOUND_EFFECT_-_MUST_USE_" 1.0 1.0 0.0 null null)
    (`self.K2_DestroyActor`)
    (bind _asmy_hud (cast `/Game/HUD/MyHUD` (`PlayerController.GetHUD` (`GameplayStatics.GetPlayerController` 0))))
    (message `/Game/Interaction/MenuInterface.Fail` _asmy_hud)
    (`KismetSystemLibrary.PrintString` "FUCK")))

(event `Key|Right`
  (params (Key :type "Key Structure"))
  ;[1 1 1] Rotation Input
  (:`Pressed`
    (set `self.Rotate` true)
    (set `self.Rotate Direction` "Z"))
  (:`Released`
    (set `self.Rotate` false)))

(event `Key|Left`
  (params (Key :type "Key Structure"))
  ;[1 1 1] Rotation Input
  (:`Pressed`
    (set `self.Rotate` true)
    (set `self.Rotate Direction` "-Z"))
  (:`Released`
    (set `self.Rotate` false)))

(event `self.ReceiveTick`
  (params (DeltaSeconds :type "Float (single-precision)"))
  (bind (_worldlocation _worlddirection) (`PlayerController.DeprojectMousePositionToWorld` (`GameplayStatics.GetPlayerController` 0)))
  ;[1 1 1] Set location
  (`|ExecutionSequence`
    (:`then_0`
      (if (`self.Rotate`)
        (`self.SetRotationDirection`)))
    (:`then_1`
      (if (`self.Active`)
        (`self.K2_SetActorLocationAndRotation` (+ _worldlocation (* _worlddirection (`self.Current offset`))) (`self.Total Rotation`))))))

(event `Key|MouseScrollUp`
  (params (Key :type "Key Structure"))
  ;[1 1 1] Movement inputs
  (:`Pressed`
    (set `self.Current offset` (+ (`self.Current offset`) 10.0))))

(event `Key|Down`
  (params (Key :type "Key Structure"))
  ;[1 1 1] Rotation Input
  (:`Pressed`
    (set `self.Rotate` true)
    (set `self.Rotate Direction` "-Y"))
  (:`Released`
    (set `self.Rotate` false)))

(event `Key|Up`
  (params (Key :type "Key Structure"))
  ;[1 1 1] Rotation Input
  (:`Pressed`
    (set `self.Rotate` true)
    (set `self.Rotate Direction` "Y"))
  (:`Released`
    (set `self.Rotate` false)))

(event `Key|MouseScrollDown`
  (params (Key :type "Key Structure"))
  ;[1 1 1] Movement inputs
  (:`Pressed`
    (set `self.Current offset` (+ (`self.Current offset`) -10.0))))

(event `Key|K`
  (params (Key :type "Key Structure"))
  ;[1 1 1] Rotation Input
  (:`Pressed`
    (set `self.Rotate` true)
    (set `self.Rotate Direction` "X"))
  (:`Released`
    (set `self.Rotate` false)))

(event `Key|L`
  (params (Key :type "Key Structure"))
  ;[1 1 1] Rotation Input
  (:`Pressed`
    (set `self.Rotate` true)
    (set `self.Rotate Direction` "-X"))
  (:`Released`
    (set `self.Rotate` false)))

(event `self.Cube.OnClicked`
  (params (TouchedComponent :type "PrimitiveComponent Object Reference") (ButtonPressed :type "Key Structure"))
  ;[1 1 1] Select and hover over
  (if (`self.Active`)
    (set `self.Active` false)
    (set `self.Current offset` 500.0)
    (`GameplayStatics.PlaySound2D` "/Game/Audio/hammering_-_sound_effect__1_.hammering_-_sound_effect__1_" 1.0 1.0 0.0 null null)
    (else
      (set `self.Active` true)
      (`self.EnableInput` (`GameplayStatics.GetPlayerController` 0))
      (`KismetSystemLibrary.PrintString` "input enabled"))))

(event `self.Cube.OnComponentBeginOverlap`
  (params (OverlappedComponent :type "PrimitiveComponent Object Reference") (OtherActor :type "Actor Object Reference") (OtherComp :type "PrimitiveComponent Object Reference") (OtherBodyIndex :type Integer) (bFromSweep :type Boolean) (SweepResult :type "HitResult Structure (by ref)"))
  ;[1 1 1] Notify player of overlap
  (bind _ignore_ (`self.Ignore` (`GameplayStatics.GetObjectClass` OtherActor)))
  (if (not _ignore_)
    (`PrimitiveComponent.SetMaterial` (`self.Cube`) 0 "/Game/StarterContent/Materials/RedMetal.RedMetal")
    (set `self.Overlap` true)))

(event `self.Cube.OnComponentEndOverlap`
  (params (OverlappedComponent :type "PrimitiveComponent Object Reference") (OtherActor :type "Actor Object Reference") (OtherComp :type "PrimitiveComponent Object Reference") (OtherBodyIndex :type Integer))
  (bind _cube (`self.Cube`))
  ;[1 1 1] Notify player of overlap
  (if (`KismetStringLibrary.EqualEqual_StrStr` (`self.Previous material`) "Green")
    (`PrimitiveComponent.SetMaterial` _cube 0 "/Game/StarterContent/Materials/GreenMetal.GreenMetal")
    (set `self.Overlap` false)
    (else
      (`PrimitiveComponent.SetMaterial` _cube 0 "/Game/StarterContent/Materials/M_Metal_Brushed_Nickel.M_Metal_Brushed_Nickel")
      (set `self.Overlap` false))))

(event `self.Cube.OnBeginCursorOver`
  (params (TouchedComponent :type "PrimitiveComponent Object Reference"))
  ;[1 1 1] Select and hover over
  (if (`self.Overlap`)
    (if (not (`self.Active`))
      (`PrimitiveComponent.SetMaterial` (`self.Cube`) 0 "/Game/StarterContent/Materials/GreenMetal.GreenMetal" :!label _label)
      (set `self.Previous material` "Green"))
    (else
      (goto _label))))

(event `self.Cube.OnEndCursorOver`
  (params (TouchedComponent :type "PrimitiveComponent Object Reference"))
  (bind _cube (`self.Cube`))
  ;[1 1 1] Select and hover over
  (if (`self.Active`)
    _
    (else
      _))
  (if (`self.Overlap`)
    (`PrimitiveComponent.SetMaterial` _cube 0 "/Game/StarterContent/Materials/RedMetal.RedMetal")
    (else
      (`PrimitiveComponent.SetMaterial` _cube 0 "/Game/StarterContent/Materials/M_Metal_Brushed_Nickel.M_Metal_Brushed_Nickel")))
  (set `self.Previous material` "Normal"))

(fn `CalcTotalRotation`)

(fn `Ignore`
  (params (Hit :type "Actor Class Reference"))
  (returns (`ignore?` :type Boolean))
  (`|ExecutionSequence`
    (:`then_0`
      (if (== Hit "/Game/Blueprints/Limiter.Limiter_C")
        (set `self.ignore?` true)
        (return (`self.ignore?`))))
    (:`then_1`
      (if (== Hit "/Game/Blueprints/Floor_Hitbox.Floor_Hitbox_C")
        (set `self.ignore?` true)
        (return (`self.ignore?`))))
    (:`then_2`
      (if (== Hit "/Game/Blueprints/LightFall.LightFall_C")
        (set `self.ignore?` true)
        (return (`self.ignore?`))))
    (:`then_3`
      (if (== Hit "/Game/Blueprints/MediumFall.MediumFall_C")
        (set `self.ignore?` true)
        (return (`self.ignore?`))))
    (:`then_4`
      (if (== Hit "/Game/Blueprints/HeavyFall.HeavyFall_C")
        (set `self.ignore?` true)
        (return (`self.ignore?`))))
    (:`then_5`
      (set `self.ignore?` false)
      (return (`self.ignore?`)))))

(fn `SetRotationDirection`
  ;[1 1 1] X
  (if (`KismetStringLibrary.EqualEqual_StrStr` (`self.Rotate Direction`) "X")
    (set `self.Total Rotation` (`KismetMathLibrary.MakeRotator` (+ (.roll (`self.Total Rotation`)) 1.0) (.pitch (`self.Total Rotation`)) (.yaw (`self.Total Rotation`))))
    (else
      ;[1 1 1] Y
      (if (`KismetStringLibrary.EqualEqual_StrStr` (`self.Rotate Direction`) "Y")
        (set `self.Total Rotation` (`KismetMathLibrary.MakeRotator` (.roll (`self.Total Rotation`)) (+ (.pitch (`self.Total Rotation`)) 1.0) (.yaw (`self.Total Rotation`))))
        (else
          ;[1 1 1] Z
          (if (`KismetStringLibrary.EqualEqual_StrStr` (`self.Rotate Direction`) "Z")
            (set `self.Total Rotation` (`KismetMathLibrary.MakeRotator` (.roll (`self.Total Rotation`)) (.pitch (`self.Total Rotation`)) (+ (.yaw (`self.Total Rotation`)) 1.0)))
            (else
              ;[1 1 1] -X
              (if (`KismetStringLibrary.EqualEqual_StrStr` (`self.Rotate Direction`) "-X")
                (set `self.Total Rotation` (`KismetMathLibrary.MakeRotator` (- (.roll (`self.Total Rotation`)) 1.0) (.pitch (`self.Total Rotation`)) (.yaw (`self.Total Rotation`))))
                (else
                  ;[1 1 1] -Y
                  (if (`KismetStringLibrary.EqualEqual_StrStr` (`self.Rotate Direction`) "-Y")
                    (set `self.Total Rotation` (`KismetMathLibrary.MakeRotator` (.roll (`self.Total Rotation`)) (- (.pitch (`self.Total Rotation`)) 1.0) (.yaw (`self.Total Rotation`))))
                    (else
                      ;[1 1 1] -Z
                      (set `self.Total Rotation` (`KismetMathLibrary.MakeRotator` (.roll (`self.Total Rotation`)) (.pitch (`self.Total Rotation`)) (- (.yaw (`self.Total Rotation`)) 1.0))))))))))))))

(fn `UserConstructionScript`)