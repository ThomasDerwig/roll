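; Snapping function that takes an object location, apparently to snap it to a one-unit grid.
; It rounds each of X, Y and Z to the nearest whole number.
; The rounded values feed CreateVectorFromYawPitch as yaw, pitch and length rather than a plain vector, so the result is a direction scaled by Z, not a snapped position.
; The other object's location and size inputs are unused.
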(fn `Snapping`
  (params (`Obj Location` :type "Vector Structure") (`Other Object Location` :type "Vector Structure") (`Othe Object Size` :type "Vector Structure"))
  (returns (`Snapped Coord` :type "Vector Structure"))
  (return (`KismetMathLibrary.CreateVectorFromYawPitch` (* (`KismetMathLibrary.Conv_IntToDouble` (`KismetMathLibrary.Round` (/ (.x `Obj Location`) 1.0))) 1.0) (* (`KismetMathLibrary.Conv_IntToDouble` (`KismetMathLibrary.Round` (/ (.y `Obj Location`) 1.0))) 1.0) (* (`KismetMathLibrary.Conv_IntToDouble` (`KismetMathLibrary.Round` (/ (.z `Obj Location`) 1.0))) 1.0))))