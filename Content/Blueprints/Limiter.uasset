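; Limiter is a box trigger actor that reports a failure on the player's HUD when nothing is inside it.
; Box begin and end overlap events add and remove actors in a tracked list, with removal printing a debug result.
; Its Start event checks whether that list is empty and, if so, casts the first player's HUD to MyHUD and calls FailMessage.
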(event `/Game/Interaction/MenuInterface.Start`
  (if (not (>= (`KismetArrayLibrary.Array_LastIndex` (`.List_3_AF8C3D384AAA7BF7E4153B93A13BFF35` (break `/DatasmithContent/Blueprints/FBXImporter/ArrayOfActor` (`self.Overlapped Components`)))) 0))
    (bind _asmy_hud (cast `/Game/HUD/MyHUD` (`PlayerController.GetHUD` (`GameplayStatics.GetPlayerController` 0))))
    (message `/Game/Interaction/MenuInterface.Fail` _asmy_hud)))

(event `self.Box.OnComponentBeginOverlap`
  (params (OverlappedComponent :type "PrimitiveComponent Object Reference") (OtherActor :type "Actor Object Reference") (OtherComp :type "PrimitiveComponent Object Reference") (OtherBodyIndex :type Integer) (bFromSweep :type Boolean) (SweepResult :type "HitResult Structure (by ref)"))
  (`KismetArrayLibrary.Array_Add` (`.List_3_AF8C3D384AAA7BF7E4153B93A13BFF35` (break `/DatasmithContent/Blueprints/FBXImporter/ArrayOfActor` (`self.Overlapped Components`))) OtherActor))

(event `self.Box.OnComponentEndOverlap`
  (params (OverlappedComponent :type "PrimitiveComponent Object Reference") (OtherActor :type "Actor Object Reference") (OtherComp :type "PrimitiveComponent Object Reference") (OtherBodyIndex :type Integer))
  (bind _returnvalue (`KismetArrayLibrary.Array_RemoveItem` (`.List_3_AF8C3D384AAA7BF7E4153B93A13BFF35` (break `/DatasmithContent/Blueprints/FBXImporter/ArrayOfActor` (`self.Overlapped Components`))) OtherActor))
  (if _returnvalue
    (`KismetSystemLibrary.PrintString` "True")
    (else
      (`KismetSystemLibrary.PrintString` "False"))))

(fn `UserConstructionScript`)