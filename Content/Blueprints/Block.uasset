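; Block is a wooden cube actor the player clicks to pick up, position and rotate, and that can break under accumulated weight.
; While active it follows the deprojected mouse each Tick at a wheel-adjusted distance, with arrow keys spinning it per axis via SetRotationDirection.
; Cursor hover and overlap events swap its material between oak, green and orange.
; RegisterHit sums incoming weight and triggers MyHUD's fail message past BreakLimit.
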(event `/Game/Interaction/Hit.Register hit`
  (params (Weight :type Integer))
  ;[1 1 1] Break
  (bind _output_get (set `self.Current break` (+ Weight (`self.Current break`))))
  (`KismetSystemLibrary.PrintString` (`KismetStringLibrary.Conv_IntToString` (`self.Current break`)))
  (if (> _output_get (`self.Break Limit`))
    (bind _asmy_hud (cast `/Game/HUD/MyHUD` (`PlayerController.GetHUD` (`GameplayStatics.GetPlayerController` 0))))
    (message `/Game/Interaction/MenuInterface.Fail` _asmy_hud)))

(event `Key|Right`
  (params (Key :type "Key Structure"))
  ;[1 1 1] Rotation Input
  (:`Pressed`
    (set `self.Rotate` true)
    (set `self.Rotate Direction` "X"))
  (:`Released`
    (set `self.Rotate` false)))

(event `self.ReceiveTick`
  (params (DeltaSeconds :type "Float (single-precision)"))
  (bind (_worldlocation _worlddirection) (`PlayerController.DeprojectMousePositionToWorld` (`GameplayStatics.GetPlayerController` 0)))
  ;[1 1 1] Set location
  (`|ExecutionSequence`
    (:`then_0`
      (if (`self.Rotate`)
        (`self.SetRotationDirection`)))
    (:`then_1`
      (if (`self.Active`)
        (`self.K2_SetActorLocationAndRotation` (+ _worldlocation (* _worlddirection (`self.Current offset`))) (`self.Total Rotation`))))))

(event `Key|MouseScrollUp`
  (params (Key :type "Key Structure"))
  ;[1 1 1] Movement inputs
  (:`Pressed`
    (set `self.Current offset` (+ (`self.Current offset`) 10.0))))

(event `Key|Left`
  (params (Key :type "Key Structure"))
  ;[1 1 1] Rotation Input
  (:`Pressed`
    (set `self.Rotate` true)
    (set `self.Rotate Direction` "Z"))
  (:`Released`
    (set `self.Rotate` false)))

(event `Key|Up`
  (params (Key :type "Key Structure"))
  ;[1 1 1] Rotation Input
  (:`Pressed`
    (set `self.Rotate` true)
    (set `self.Rotate Direction` "Y"))
  (:`Released`
    (set `self.Rotate` false)))

(event `Key|MouseScrollDown`
  (params (Key :type "Key Structure"))
  ;[1 1 1] Movement inputs
  (:`Pressed`
    (set `self.Current offset` (+ (`self.Current offset`) -10.0))))

(event `self.Cube.OnClicked`
  (params (TouchedComponent :type "PrimitiveComponent Object Reference") (ButtonPressed :type "Key Structure"))
  ;[1 1 1] Select and hover over
  (if (`self.Active`)
    (set `self.Active` false)
    (set `self.Current offset` 500.0)
    (else
      (set `self.Active` true)
      (`self.EnableInput` (`GameplayStatics.GetPlayerController` 0))
      (`KismetSystemLibrary.PrintString` "input enabled"))))

(event `self.Cube.OnComponentBeginOverlap`
  (params (OverlappedComponent :type "PrimitiveComponent Object Reference") (OtherActor :type "Actor Object Reference") (OtherComp :type "PrimitiveComponent Object Reference") (OtherBodyIndex :type Integer) (bFromSweep :type Boolean) (SweepResult :type "HitResult Structure (by ref)"))
  (bind _returnvalue (`GameplayStatics.GetObjectClass` OtherActor))
  ;[1 1 1] Notify player of overlap
  (if (!= _returnvalue "/Game/Blueprints/Limiter.Limiter_C")
    (if (!= _returnvalue "/Game/Blueprints/Floor_Hitbox.Floor_Hitbox_C")
      (`PrimitiveComponent.SetMaterial` (`self.Cube`) 0 "/Game/StarterContent/Materials/Orange_Wood.Orange_Wood")
      (set `self.Overlap` true))))

(event `self.Cube.OnComponentEndOverlap`
  (params (OverlappedComponent :type "PrimitiveComponent Object Reference") (OtherActor :type "Actor Object Reference") (OtherComp :type "PrimitiveComponent Object Reference") (OtherBodyIndex :type Integer))
  (bind _cube (`self.Cube`))
  ;[1 1 1] Notify player of overlap
  (if (`KismetStringLibrary.EqualEqual_StrStr` (`self.Previous material`) "Green")
    (`PrimitiveComponent.SetMaterial` _cube 0 "/Game/StarterContent/Materials/Green_Wood.Green_Wood")
    (set `self.Overlap` false)
    (else
      (`PrimitiveComponent.SetMaterial` _cube 0 "/Game/StarterContent/Materials/M_Wood_Oak.M_Wood_Oak")
      (set `self.Overlap` false))))

(event `self.Cube.OnBeginCursorOver`
  (params (TouchedComponent :type "PrimitiveComponent Object Reference"))
  ;[1 1 1] Select and hover over
  (if (`self.Overlap`)
    (if (not (`self.Active`))
      (`PrimitiveComponent.SetMaterial` (`self.Cube`) 0 "/Game/StarterContent/Materials/Green_Wood.Green_Wood" :!label _label)
      (set `self.Previous material` "Green"))
    (else
      (goto _label))))

(event `self.Cube.OnEndCursorOver`
  (params (TouchedComponent :type "PrimitiveComponent Object Reference"))
  (bind _cube (`self.Cube`))
  ;[1 1 1] Select and hover over
  (if (`self.Active`)
    _
    (else
      _))
  (if (`self.Overlap`)
    (`PrimitiveComponent.SetMaterial` _cube 0 "/Game/StarterContent/Materials/Orange_Wood.Orange_Wood")
    (else
      (`PrimitiveComponent.SetMaterial` _cube 0 "/Game/StarterContent/Materials/M_Wood_Oak.M_Wood_Oak")))
  (set `self.Previous material` "Normal"))

(fn `CalcTotalRotation`)

(fn `SetRotationDirection`
  ;[1 1 1] X
  (if (`KismetStringLibrary.EqualEqual_StrStr` (`self.Rotate Direction`) "X")
    (set `self.Total Rotation` (`KismetMathLibrary.MakeRotator` (+ (.roll (`self.Total Rotation`)) 1.0) (.pitch (`self.Total Rotation`)) (.yaw (`self.Total Rotation`))))
    (else
      ;[1 1 1] Y
      (if (`KismetStringLibrary.EqualEqual_StrStr` (`self.Rotate Direction`) "Y")
        (set `self.Total Rotation` (`KismetMathLibrary.MakeRotator` (.roll (`self.Total Rotation`)) (+ (.pitch (`self.Total Rotation`)) 1.0) (.yaw (`self.Total Rotation`))))
        (else
          ;[1 1 1] Z
          (set `self.Total Rotation` (`KismetMathLibrary.MakeRotator` (.roll (`self.Total Rotation`)) (.pitch (`self.Total Rotation`)) (+ (.yaw (`self.Total Rotation`)) 1.0))))))))

(fn `UserConstructionScript`)