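; Swamp Blueprint with a Box trigger that reacts to NonOgre objects entering or leaving the area.
; End overlap by a NonOgre actor sets the Wind flag, waits briefly, then calls YayMessage on the first player's MyHUD.
; Begin overlap clears Wind, but tests the class of the overlapping component rather than the actor.
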(event `self.Box.OnComponentEndOverlap`
  (params (OverlappedComponent :type "PrimitiveComponent Object Reference") (OtherActor :type "Actor Object Reference") (OtherComp :type "PrimitiveComponent Object Reference") (OtherBodyIndex :type Integer))
  (if (== (`GameplayStatics.GetObjectClass` OtherActor) "/Game/Blueprints/NonOgre.NonOgre_C")
    (set `self.wind` true)
    (`KismetSystemLibrary.Delay` 1.0)
    (bind _asmy_hud (cast `/Game/HUD/MyHUD` (`PlayerController.GetHUD` (`GameplayStatics.GetPlayerController` 0))))
    (message `/Game/Interaction/MenuInterface.Yay` _asmy_hud)))

(event `self.Box.OnComponentBeginOverlap`
  (params (OverlappedComponent :type "PrimitiveComponent Object Reference") (OtherActor :type "Actor Object Reference") (OtherComp :type "PrimitiveComponent Object Reference") (OtherBodyIndex :type Integer) (bFromSweep :type Boolean) (SweepResult :type "HitResult Structure (by ref)"))
  (if (== (`GameplayStatics.GetObjectClass` OtherComp) "/Game/Blueprints/NonOgre.NonOgre_C")
    (set `self.wind` false)))

(fn `UserConstructionScript`)